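; BP_Player is a player Blueprint that handles basic axis-driven movement and turning.
; MoveForward and MoveRight add movement input along the actor's forward and right vectors, while Turn adds controller yaw scaled by TurnRate and delta seconds.
; Tick prints actor and controller yaw side by side for debugging.
; Pitch, roll and direct SetActorRotation nodes are left unconnected and never run.
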(event `self.ReceiveTick`
  (params (DeltaSeconds :type "Float (single-precision)"))
  (bind (_returnvalue_roll _returnvalue_pitch _returnvalue_yaw) (`KismetMathLibrary.BreakRotator` (`self.K2_GetActorRotation`)))
  (bind (_returnvalue_roll_2 _returnvalue_pitch_2 _returnvalue_yaw_2) (`KismetMathLibrary.BreakRotator` (`self.K2_GetActorRotation` (`self.GetController`))))
  (`KismetSystemLibrary.PrintText` (`|FormatText` "Player({0}) Controller({1})" _returnvalue_yaw _returnvalue_yaw_2)))

(event `InputAxis|MoveForward`
  (params (AxisValue :type "Float (single-precision)"))
  (`self.AddMovementInput` (`self.GetActorForwardVector`) AxisValue))

(event `InputAxis|MoveRight`
  (params (AxisValue :type "Float (single-precision)"))
  (`self.AddMovementInput` (`self.GetActorRightVector`) AxisValue))

(event `InputAxis|Turn`
  (params (AxisValue :type "Float (single-precision)"))
  (`self.AddControllerYawInput` (* (`self.TurnRate`) (`GameplayStatics.GetWorldDeltaSeconds`) AxisValue)))

(fn `UserConstructionScript`)