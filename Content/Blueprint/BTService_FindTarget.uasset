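; Behavior tree service that finds the player as a target for an AI-controlled pawn.
; On each AI tick it looks up the BP_Player actor with GetActorOfClass and measures its distance to the pawn.
; It writes the player to the Target blackboard key when within Range and clears the key otherwise.
; If no valid player is found, the key is left unchanged.
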(event `self.ReceiveTickAI`
  (params (OwnerController :type "AIController Object Reference") (ControlledPawn :type "Pawn Object Reference") (DeltaSeconds :type "Float (single-precision)"))
  (bind _returnvalue (`GameplayStatics.GetActorOfClass` "/Game/Blueprint/BP_Player.BP_Player_C"))
  (`/Engine/EditorBlueprintResources/StandardMacros.IsValid` _returnvalue
    (:`Is Valid`
      (if (< (`KismetMathLibrary.VSize` (- (`Actor.K2_GetActorLocation` _returnvalue) (`Actor.K2_GetActorLocation` ControlledPawn))) (`self.Range`))
        (`BTFunctionLibrary.SetBlackboardValueAsObject` (`self.Target`) _returnvalue)
        (else
          (`BTFunctionLibrary.SetBlackboardValueAsObject` (`self.Target`)))))))